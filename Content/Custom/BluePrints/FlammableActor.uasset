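; FlammableActor is an actor that feeds its fire level, PercentOnFire, into the player's score.
; On every Tick it casts player 0's character to ThirdPersonCharacter and adds PercentOnFire to PlayerScore, so the gain depends on frame rate.
; A one-second Delay after the addition throttles only the debug print of PercentOnFire.
; A threshold check on PercentOnFire is left unconnected and never runs.
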(event `self.ReceiveTick`
  (params (DeltaSeconds :type "Float (single-precision)"))
  (bind _percentonfire (`self.PercentOnFire`))
  (bind _asthird_person_character (cast `/Game/Custom/BluePrints/ThirdPersonCharacter` (`GameplayStatics.GetPlayerCharacter` 0)))
  (set `/Game/Custom/BluePrints/ThirdPersonCharacter.PlayerScore` (+ (`/Game/Custom/BluePrints/ThirdPersonCharacter.PlayerScore` _asthird_person_character) _percentonfire) _asthird_person_character)
  (`KismetSystemLibrary.Delay` 1.0)
  (`KismetSystemLibrary.PrintString` (`KismetStringLibrary.Conv_DoubleToString` _percentonfire)))

(fn `UserConstructionScript`)